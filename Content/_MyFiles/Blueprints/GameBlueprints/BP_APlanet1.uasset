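; BP_APlanet1 is a planet actor that sizes its visuals and gravity field from a single Radius.
; UpdatePlanet scales the sphere mesh, computes GravityFieldRadius slightly larger than Radius in scaled units, and hides the sphere in game when IsClosetPlanet (apparently "closest") is set.
; For that planet, it also scales any valid VoxelWorld and Atmosphere and moves them to its location.
; GetGravityRadius exposes the field radius; the event graph is unused.
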(fn `GetGravityRadius`
  (returns (GravityRadius :type "Float (double-precision)"))
  (return (`self.GravityFieldRadius`)))

(fn `UpdatePlanet`
  (`SceneComponent.SetWorldScale3D` (`self.PlanetSphere`) (`KismetMathLibrary.Conv_DoubleToVector` (* (`self.Radius`) 2.0 1000.0)))
  (set `self.GravityFieldRadius` (* (`self.Radius`) 1.1 100000.0))
  (`SceneComponent.SetHiddenInGame` (`self.PlanetSphere`) (`self.IsClosetPlanet`) false)
  (if (`self.IsClosetPlanet`)
    (`|ExecutionSequence`
      (:`then_0`
        (bind _voxelworld (`self.VoxelWorld`)
          (:`then`
            (`self.SetActorScale3D` _voxelworld (`KismetMathLibrary.Conv_DoubleToVector` (`self.Radius`)))
            (`self.K2_SetActorLocation` _voxelworld (`self.K2_GetActorLocation`) false false))
          (:`else`)))
      (:`then_1`
        (bind _atmosphere (`self.Atmosphere`)
          (:`then`
            (`self.SetActorScale3D` _atmosphere (`KismetMathLibrary.Conv_DoubleToVector` (`self.Radius`)))
            (`self.K2_SetActorLocation` _atmosphere (`self.K2_GetActorLocation`) false false))
          (:`else`))))))

(fn `UserConstructionScript`)